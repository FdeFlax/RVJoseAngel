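; BP_Weapon is a VR weapon that can be picked up, dropped and fired.
; A grab sphere tracks the overlapping BP_VRPlayer, while PickUp records the holder, snaps to its right motion controller and disables mesh physics.
; Drop clears the held state and detaches in world space, while Reset only detaches.
; Fire spawns a BP_Projectile at the ShootOrigin's location and rotation.
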(event OnComponentBeginOverlap(GrabSphere)
  (params (OverlappedComponent :type Primitive%20Component%20Object%20Reference) (OtherActor :type Actor%20Object%20Reference) (OtherComp :type Primitive%20Component%20Object%20Reference) (OtherBodyIndex :type Integer) (bFromSweep :type Boolean) (SweepResult :type Hit%20Result%20Structure%20%28by%20ref%29))
  (bind _asbp_vrplayer (Utilities|Casting|CastToBP_VRPlayer OtherActor))
  (Variables|Default|SetOverlappingPlayer _asbp_vrplayer))

(event OnComponentEndOverlap(GrabSphere)
  (params (OverlappedComponent :type Primitive%20Component%20Object%20Reference) (OtherActor :type Actor%20Object%20Reference) (OtherComp :type Primitive%20Component%20Object%20Reference) (OtherBodyIndex :type Integer))
  (Utilities|Casting|CastToBP_VRPlayer OtherActor)
  (Variables|Default|SetOverlappingPlayer 0))

(event Custom|PickUp
  (params (Grabber :type BP%20VR%20Player%20Object%20Reference))
  (Variables|Default|SetblsHeld true)
  (Variables|Default|SetHeldBy Grabber)
  (Transformation|AttachComponentToComponent (Variables|/Game/Game/BP/BP_VRPlayer.BP_VRPlayer_C|GetMotionController_Right Grabber) "None" "SnapToTarget" "SnapToTarget" "SnapToTarget" false)
  (Physics|SetSimulatePhysics (Variables|Default|GetMesh_Weapon) false))

(event Custom|Fire
  (bind _shootorigin (Variables|Default|GetShootOrigin))
  (Game|SpawnActorfromClass "/Game/Game/BP/BP_Projectile.BP_Projectile_C" (Math|Transform|MakeTransform (Transformation|GetWorldLocation _shootorigin) (Transformation|GetWorldRotation _shootorigin) "1.000000,1.000000,1.000000") "Undefined" "MultiplyWithRoot" 0 0))

(event Custom|DropWeapon
  (Variables|Default|SetblsHeld false)
  (Variables|Default|SetHeldBy 0)
  (Transformation|DetachFromActor "KeepWorld" "KeepWorld" "KeepWorld"))

(event Custom|ResetWeapon
  (Transformation|DetachFromActor "KeepWorld" "KeepWorld" "KeepWorld"))

(fn ConstructionScript)