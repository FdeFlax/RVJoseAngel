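; BP_Menu is a VR menu actor that displays WBP_Master on a widget component and takes pointer clicks from the player.
; On BeginPlay it caches the VR player pawn, enables its tick and input, and adds an Enhanced Input mapping context.
; IA_UI_Click presses and releases left mouse through the pawn's right-hand widget interaction component.
; The actor destroys itself when the nested WBPMenu fires its DeleteWidget dispatcher.
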(event Custom|DeleteWidget_Event
  (Actor|DestroyActor))

(event Input|EnhancedActionEvents|EnhancedInputActionIA_UI_Click
  (params (ActionValue :type Boolean) (ElapsedSeconds :type Float%20%28double-precision%29) (TriggeredSeconds :type Float%20%28double-precision%29) (InputAction :type Input%20Action%20Object%20Reference :default "/Game/Game/BP/IA_UI_Click.IA_UI_Click"))
  (bind _vrpawn (Variables|Default|GetVRPawn))
  (bind _widgetinteraction_right (Variables|/Game/Game/BP/BP_VRPlayer.BP_VRPlayer_C|GetWidgetInteraction_Right _vrpawn))
  (:Triggered
    (Class|WidgetInteractionComponent|PressPointerKey _widgetinteraction_right "LeftMouseButton"))
  (:Canceled
    (Class|WidgetInteractionComponent|ReleasePointerKey _widgetinteraction_right "LeftMouseButton" :!label _label))
  (:Completed
    (goto _label)))

(event EventBeginPlay
  (bind _returnvalue (Game|GetPlayerController 0))
  (bind _asbp_vrplayer (Utilities|Casting|CastToBP_VRPlayer (Game|Player|GetPlayerPawn 0)))
  (bind _output_get (Variables|Default|SetVRPawn _asbp_vrplayer))
  (Actor|Tick|SetActorTickEnabled _output_get true)
  (Input|EnableInput _returnvalue)
  (Input|AddMappingContext (PlayerController|LocalPlayerSubsystems|GetEnhancedInputLocalPlayerSubsystem _returnvalue) 0 1 "(bIgnoreAllPressedKeysUntilRelease=True,bForceImmediately=False,bNotifyUserSettings=False)")
  (bind _aswbp_master (Utilities|Casting|CastToWBP_Master (UserInterface|GetWidget (Variables|Default|GetWidget))))
  (EventDispatchers|AssignDeleteWidget (Variables|/Game/Game/BP/WBP_Master.WBP_Master_C|GetWBP_Menu _aswbp_master) (delegate Custom|DeleteWidget_Event)))

(fn ConstructionScript)