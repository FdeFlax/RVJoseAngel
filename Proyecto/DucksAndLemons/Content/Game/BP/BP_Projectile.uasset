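; Projectile for a VR target-shooting game that scores hits on positive and negative targets.
; Sphere overlap with BP_TargetObject plays a sound, adds a point through BP_VRGameMode, destroys the projectile and notifies the first BP_Spawner with a fixed shot index.
; Overlap with BP_TargetNegative plays another sound, subtracts a point and destroys both actors without notifying the spawner.
; Physical hits only print the actor's name.
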(event OnComponentHit(Sphere)
  (params (HitComponent :type Primitive%20Component%20Object%20Reference) (OtherActor :type Actor%20Object%20Reference) (OtherComp :type Primitive%20Component%20Object%20Reference) (NormalImpulse :type Vector :default "0, 0, 0") (Hit :type Hit%20Result%20Structure%20%28by%20ref%29))
  (Development|PrintString (Utilities|String|Append "Hit name:" (Utilities|GetDisplayName OtherActor))))

(event OnComponentBeginOverlap(Sphere)
  (params (OverlappedComponent :type Primitive%20Component%20Object%20Reference) (OtherActor :type Actor%20Object%20Reference) (OtherComp :type Primitive%20Component%20Object%20Reference) (OtherBodyIndex :type Integer) (bFromSweep :type Boolean) (SweepResult :type Hit%20Result%20Structure%20%28by%20ref%29))
  (Utilities|FlowControl|Sequence
    (:then_0
      (Utilities|Casting|CastToBP_TargetObject OtherActor)
      (if true
        (Audio|PlaySoundatLocation "/Game/Game/Sounds/patito.patito" "0, 0, 0" "0, 0, 0" 1.0 1.0 0.0 0 0 0 0)
        (bind _asbp_vrgame_mode (Utilities|Casting|CastToBP_VRGameMode (Game|GetGameMode)))
        (Default|AddScore _asbp_vrgame_mode 1)
        (bind _outactors (Actor|GetAllActorsOfClass "/Game/Game/BP/BP_Spawner.BP_Spawner_C"))
        (Actor|DestroyActor)
        (Default|OnTargetShot (Utilities|Array|Get(acopy) _outactors) 0 true)))
    (:then_1
      (bind _asbp_target_negative (Utilities|Casting|CastToBP_TargetNegative OtherActor))
      (if true
        (Audio|PlaySoundatLocation "/Game/Game/Sounds/mal.mal" "0, 0, 0" "0, 0, 0" 1.0 1.0 0.0 0 0 0 0)
        (bind _asbp_vrgame_mode_2 (Utilities|Casting|CastToBP_VRGameMode (Game|GetGameMode)))
        (Default|AddScore _asbp_vrgame_mode_2 -1)
        (bind _outactors_2 (Actor|GetAllActorsOfClass "/Game/Game/BP/BP_Spawner.BP_Spawner_C"))
        (Actor|DestroyActor _asbp_target_negative)
        (Actor|DestroyActor)))))

(event EventBeginPlay)

(fn ConstructionScript)