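; BP_Count is a countdown timer actor that shows the remaining seconds through its CountdownText.
; BeginPlay seeds TimeRemaining with a fixed duration, and Tick subtracts delta time and writes the value to the text with up to two decimals.
; Updates stop once the next step would reach zero or below, so the display never shows zero and no expiry action fires.
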(event EventBeginPlay
  (Variables|Default|SetTimeRemaining 125.0))

(event Collision|EventActorBeginOverlap
  (params (OtherActor :type Actor%20Object%20Reference)))

(event EventTick
  (params (DeltaSeconds :type Float%20%28single-precision%29))
  (if (not (<= (- (Variables|Default|GetTimeRemaining) DeltaSeconds) 0.0))
    (bind _output_get (Variables|Default|SetTimeRemaining (- (Variables|Default|GetTimeRemaining) DeltaSeconds)))
    (Rendering|Components|TextRender|SetText (Variables|Default|GetCountdownText) (Utilities|Text|ToText(Float) _output_get "HalfToEven" false true 1 324 0 2))))

(fn ConstructionScript)