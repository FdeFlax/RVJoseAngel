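; VR game mode that runs a timed two-minute scoring session and tracks the player's score.
; StartScoringSession opens scoring and sets a timer for EndScoringSession, which closes it, spawns BP_Menu at a fixed spot, reveals the button, hides and resets the countdown, and zeroes the display.
; AddScore accumulates and pushes totals to BP_ScoreDisplay during a session; outside one, it clears Score.
; World actors are found by class, using the first match.
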(event Custom|StartScoringSession
  (Variables|Default|SetbCanScore true)
  (Utilities|Time|SetTimerbyFunctionName 0 "EndScoringSession" 1.2e+02))

(event Custom|EndScoringSession
  (Variables|Default|SetbCanScore false)
  (Variables|Default|SetbGameStarted false)
  (Game|SpawnActorfromClass "/Game/Game/BP/BP_Menu.BP_Menu_C" (Math|Transform|MakeTransform (+ "" "110.000000,50.000000,20.000000") (Math|Conversions|RotationFromXVector (+ "" "0.000000,0.000000,20.000000")) "1.000000,1.000000,1.000000") "Undefined" "MultiplyWithRoot" 0 0)
  (bind _outactors (Actor|GetAllActorsOfClass "/Game/Game/BP/BP_Button.BP_Button_C"))
  (Rendering|SetVisibility (Variables|/Game/Game/BP/BP_Button.BP_Button_C|GetStaticMesh (Utilities|Array|Get(acopy) _outactors)) true false)
  (bind _outactors_2 (Actor|GetAllActorsOfClass "/Game/Game/BP/BP_Count.BP_Count_C"))
  (Rendering|SetVisibility (Variables|/Game/Game/BP/BP_Count.BP_Count_C|GetCountdownText (Utilities|Array|Get(acopy) _outactors_2)) false false)
  (Variables|/Game/Game/BP/BP_Count.BP_Count_C|SetTimeRemaining (Utilities|Array|Get(acopy) _outactors_2) 1.2e+02)
  (bind _outactors_3 (Actor|GetAllActorsOfClass "/Game/Game/BP/BP_ScoreDisplay.BP_ScoreDisplay_C"))
  (Default|UpdateScoreDisplay (Utilities|Array|Get(acopy) _outactors_3)))

(event Custom|GameStarted
  (Variables|Default|SetbGameStarted true))

(fn ConstructionScript)

(fn AddScore
  (params (Delta :type Integer))
  (if (Variables|Default|GetbCanScore)
    (bind _output_get (Variables|Default|SetScore (+ Delta (Variables|Default|GetScore))))
    (bind _outactors (Actor|GetAllActorsOfClass "/Game/Game/BP/BP_ScoreDisplay.BP_ScoreDisplay_C"))
    (Default|UpdateScoreDisplay (Utilities|Array|Get(acopy) _outactors) _output_get)
    (else
      (Variables|Default|SetScore 0))))