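; BP_VRPlayer is the VR player pawn or character, handling Enhanced Input movement, look, UI clicks and weapon use.
; A right-hand sphere overlap tracks the BP_Weapon in reach, which grab picks up as the held weapon for firing or dropping.
; Movement follows fixed world axes, and drop checks the in-reach weapon rather than the held one.
; Grab and fire read the game mode's GameStarted flag, but neither branch gates the action.
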(event OnComponentBeginOverlap(RightSphere)
  (params (OverlappedComponent :type Primitive%20Component%20Object%20Reference) (OtherActor :type Actor%20Object%20Reference) (OtherComp :type Primitive%20Component%20Object%20Reference) (OtherBodyIndex :type Integer) (bFromSweep :type Boolean) (SweepResult :type Hit%20Result%20Structure%20%28by%20ref%29))
  (bind _asbp_weapon (Utilities|Casting|CastToBP_Weapon OtherActor))
  (Variables|Default|SetWeaponInReach _asbp_weapon))

(event OnComponentEndOverlap(RightSphere)
  (params (OverlappedComponent :type Primitive%20Component%20Object%20Reference) (OtherActor :type Actor%20Object%20Reference) (OtherComp :type Primitive%20Component%20Object%20Reference) (OtherBodyIndex :type Integer))
  (Utilities|Casting|CastToBP_Weapon OtherActor)
  (Variables|Default|SetWeaponInReach 0))

(event Input|EnhancedActionEvents|EnhancedInputActionIA_UI_Click
  (params (ActionValue :type Boolean) (ElapsedSeconds :type Float%20%28double-precision%29) (TriggeredSeconds :type Float%20%28double-precision%29) (InputAction :type Input%20Action%20Object%20Reference :default "/Game/Game/BP/IA_UI_Click.IA_UI_Click"))
  (Class|WidgetInteractionComponent|PressPointerKey (Variables|Default|GetWidgetInteraction_Right) "LeftMouseButton"))

(event Input|EnhancedActionEvents|EnhancedInputActionIA_Fire
  (params (ActionValue :type Boolean) (ElapsedSeconds :type Float%20%28double-precision%29) (TriggeredSeconds :type Float%20%28double-precision%29) (InputAction :type Input%20Action%20Object%20Reference :default "/Game/Game/BP/IA_Fire.IA_Fire"))
  (bind _heldweapon (Variables|Default|GetHeldWeapon))
  (bind _asbp_vrgame_mode (Utilities|Casting|CastToBP_VRGameMode (Game|GetGameMode)))
  (if (Variables|/Game/Game/BP/BP_VRGameMode.BP_VRGameMode_C|GetbGameStarted _asbp_vrgame_mode)
    _
    (else
      _))
  (Utilities|IsValid _heldweapon
    (:Is%20Valid
      (if true
        (Audio|PlaySoundatLocation "/Game/Game/Sounds/proyectil.proyectil" "0, 0, 0" "0, 0, 0" 1.0 1.0 0.0 0 0 0 0)
        (Default|Fire _heldweapon)))))

(event Input|EnhancedActionEvents|EnhancedInputActionIA_Grab
  (params (ActionValue :type Boolean) (ElapsedSeconds :type Float%20%28double-precision%29) (TriggeredSeconds :type Float%20%28double-precision%29) (InputAction :type Input%20Action%20Object%20Reference :default "/Game/Game/BP/IA_Grab.IA_Grab"))
  (bind _weaponinreach (Variables|Default|GetWeaponInReach))
  (bind _asbp_vrgame_mode (Utilities|Casting|CastToBP_VRGameMode (Game|GetGameMode)))
  (if (Variables|/Game/Game/BP/BP_VRGameMode.BP_VRGameMode_C|GetbGameStarted _asbp_vrgame_mode)
    _
    (else
      _))
  (Utilities|IsValid _weaponinreach
    (:Is%20Valid
      (Default|PickUp _weaponinreach self)
      (Variables|Default|SetHeldWeapon _weaponinreach))))

(event Input|EnhancedActionEvents|EnhancedInputActionIA_Drop
  (params (ActionValue :type Boolean) (ElapsedSeconds :type Float%20%28double-precision%29) (TriggeredSeconds :type Float%20%28double-precision%29) (InputAction :type Input%20Action%20Object%20Reference :default "/Game/Game/BP/IA_Drop.IA_Drop"))
  (Utilities|IsValid (Variables|Default|GetWeaponInReach)
    (:Is%20Valid
      (Default|DropWeapon (Variables|Default|GetHeldWeapon))
      (Variables|Default|SetHeldWeapon 0))))

(event Input|EnhancedActionEvents|EnhancedInputActionIA_MoveRight
  (params (ActionValue :type Float%20%28double-precision%29) (ElapsedSeconds :type Float%20%28double-precision%29) (TriggeredSeconds :type Float%20%28double-precision%29) (InputAction :type Input%20Action%20Object%20Reference :default "/Game/Game/BP/IA_MoveRight.IA_MoveRight"))
  (Pawn|Input|AddMovementInput "0.000000,1.000000,0.000000" ActionValue false))

(event Input|EnhancedActionEvents|EnhancedInputActionIA_MoveForeward
  (params (ActionValue :type Float%20%28double-precision%29) (ElapsedSeconds :type Float%20%28double-precision%29) (TriggeredSeconds :type Float%20%28double-precision%29) (InputAction :type Input%20Action%20Object%20Reference :default "/Game/Game/BP/IA_MoveForeward.IA_MoveForeward"))
  (Pawn|Input|AddMovementInput "1.000000,0.000000,0.000000" ActionValue false))

(event Input|EnhancedActionEvents|EnhancedInputActionIA_Look
  (params (ActionValue :type Vector%202D%20Structure) (ElapsedSeconds :type Float%20%28double-precision%29) (TriggeredSeconds :type Float%20%28double-precision%29) (InputAction :type Input%20Action%20Object%20Reference :default "/Game/Game/BP/IA_Look.IA_Look"))
  (Pawn|Input|AddControllerPitchInput (* (.Y (Math|Vector2D|BreakVector2D (stale ActionValue))) -1.0)))

(event Input|EnhancedActionEvents|EnhancedInputActionIA_Look
  (params (ActionValue :type Vector%202D%20Structure) (ElapsedSeconds :type Float%20%28double-precision%29) (TriggeredSeconds :type Float%20%28double-precision%29) (InputAction :type Input%20Action%20Object%20Reference :default "/Game/Game/BP/IA_Look.IA_Look"))
  (Pawn|Input|AddControllerYawInput (.X (Math|Vector2D|BreakVector2D ActionValue))))

(event EventBeginPlay
  (bind _asplayer_controller (Utilities|Casting|CastToPlayerController (Pawn|GetController)))
  (Utilities|IsValid (PlayerController|LocalPlayerSubsystems|GetEnhancedInputLocalPlayerSubsystem _asplayer_controller)
    (:Is%20Valid
      (Input|AddMappingContext (PlayerController|LocalPlayerSubsystems|GetEnhancedInputLocalPlayerSubsystem _asplayer_controller) "/Game/Game/BP/NewInputMappingContext.NewInputMappingContext" 0 "(bIgnoreAllPressedKeysUntilRelease=True,bForceImmediately=False,bNotifyUserSettings=False)"))))

(fn ConstructionScript)