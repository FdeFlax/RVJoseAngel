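; Shootable start button that begins a scoring session in the VR game when a BP_Projectile overlaps its sphere.
; The overlap calls StartScoringSession on BP_VRGameMode and sets the countdown time on the first BP_Count found in the level.
; It then swaps the BP_Informador info display for the countdown text, hides the button mesh and destroys the projectile.
; The sphere's collision is left unchanged, and no guard prevents retriggering.
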(event OnComponentBeginOverlap(Sphere)
  (params (OverlappedComponent :type Primitive%20Component%20Object%20Reference) (OtherActor :type Actor%20Object%20Reference) (OtherComp :type Primitive%20Component%20Object%20Reference) (OtherBodyIndex :type Integer) (bFromSweep :type Boolean) (SweepResult :type Hit%20Result%20Structure%20%28by%20ref%29))
  (bind _asbp_projectile (Utilities|Casting|CastToBP_Projectile OtherActor))
  (bind _asbp_vrgame_mode (Utilities|Casting|CastToBP_VRGameMode (Game|GetGameMode)))
  (Default|StartScoringSession _asbp_vrgame_mode)
  (bind _outactors (Actor|GetAllActorsOfClass "/Game/Game/BP/BP_Count.BP_Count_C"))
  (Variables|/Game/Game/BP/BP_Count.BP_Count_C|SetTimeRemaining (Utilities|Array|Get(acopy) _outactors) 1.2e+02)
  (bind _outactors_2 (Actor|GetAllActorsOfClass "/Game/Game/BP/BP_Informador.BP_Informador_C"))
  (Rendering|SetVisibility (Variables|/Game/Game/BP/BP_Informador.BP_Informador_C|GetInformar (Utilities|Array|Get(acopy) _outactors_2)) false false)
  (Rendering|SetVisibility (Variables|/Game/Game/BP/BP_Count.BP_Count_C|GetCountdownText (Utilities|Array|Get(acopy) _outactors)) true false)
  (Rendering|SetVisibility (Variables|Default|GetStaticMesh) false false)
  (Actor|DestroyActor _asbp_projectile))

(event EventBeginPlay)

(event Collision|EventActorBeginOverlap
  (params (OtherActor :type Actor%20Object%20Reference)))

(event EventTick
  (params (DeltaSeconds :type Float%20%28single-precision%29)))

(fn ConstructionScript)