(event Custom|InitSpawns
  (bind _spawnactors (Variables|Default|GetSpawnActors))
  (bind _output_get (Variables|Default|SetPositiveIndex (Math|Random|RandomIntegerinRange 0 5)))
  (Development|PrintString (Utilities|String|Append "PsitiveIndex=" (Utilities|String|ToString(Integer) _output_get)))
  (for _index (range 0 5)
    (if (== _index (Variables|Default|GetPositiveIndex))
      (bind _returnvalue (Game|SpawnActorfromClass "/Game/Game/BP/BP_TargetObject.BP_TargetObject_C" (Math|Transform|MakeTransform (Utilities|Array|Get(acopy) (Variables|Default|GetSpawnPoints) _index) "0, 0, 0" "1.000000,1.000000,1.000000") "Undefined" "MultiplyWithRoot" 0 0))
      (Utilities|Array|Add _spawnactors _returnvalue)
      (else
        (bind _returnvalue_2 (Game|SpawnActorfromClass "/Game/Game/BP/BP_TargetNegative.BP_TargetNegative_C" (Math|Transform|MakeTransform (Utilities|Array|Get(acopy) (Variables|Default|GetSpawnPoints) _index) "0, 0, 0" "1.000000,1.000000,1.000000") "Undefined" "MultiplyWithRoot" 0 0))
        (Utilities|Array|Add _spawnactors _returnvalue_2)))))

(event Custom|SpawnTarget
  (bind _returnvalue (Math|Random|RandomIntegerinRange 0 4))
  (bind _array (Utilities|Array|MakeArray "ObjectTypeQuery1" "ObjectTypeQuery2"))
  (bind _spawnpoints (Variables|Default|GetSpawnPoints))
  (bind _output (Utilities|Array|Get(acopy) _spawnpoints _returnvalue))
  (if (< (Math|Random|RandomFloatinRange 0.0 1.0) 0.7)
    (bind _outactors (Collision|SphereOverlapActors _output 0.1 _array "/Script/Engine.Actor"))
    (if (== (Utilities|Array|Length _outactors) 0)
      (bind _returnvalue_2 (Game|SpawnActorfromClass "/Game/Game/BP/BP_TargetObject.BP_TargetObject_C" (Math|Transform|MakeTransform _output "0, 0, 0" "1.000000,1.000000,1.000000") "Undefined" "MultiplyWithRoot" 0 0))
      (Actor|SetLifeSpan _returnvalue_2 5.0))
    (else
      (bind _outactors_2 (Collision|SphereOverlapActors _output 0.1 _array "/Script/Engine.Actor"))
      (if (== (Utilities|Array|Length _outactors_2) 0)
        (bind _returnvalue_3 (Game|SpawnActorfromClass "/Game/Game/BP/BP_TargetNegative.BP_TargetNegative_C" (Math|Transform|MakeTransform _output "0, 0, 0" "1.000000,1.000000,1.000000") "Undefined" "MultiplyWithRoot" 0 0))
        (Actor|SetLifeSpan _returnvalue_3 5.0)))))

(event Custom|OnTargetShot
  (params (ShotIndex :type Integer) (WasPositive :type Boolean))
  (bind _spawnactors (Variables|Default|GetSpawnActors))
  (Development|PrintString (Utilities|String|Append " Index=" (Utilities|String|ToString(Integer) ShotIndex) "Was Positve" (Utilities|String|ToString(Boolean) WasPositive)))
  (if WasPositive
    (for _array_element _spawnactors
      (Utilities|IsValid _array_element
        (:Is%20Valid
          (Actor|DestroyActor _array_element))))
    (Utilities|Array|Clear _spawnactors)
    (CallFunction|InitSpawns)))

(event EventBeginPlay
  (CallFunction|InitSpawns))

(fn ConstructionScript
  (Components|InstancedStaticMesh|ClearInstances (Variables|Default|GetPreviewSpheres))
  (for _array_element (Variables|Default|GetSpawnPoints)
    (Components|InstancedStaticMesh|AddInstance (Variables|Default|GetPreviewSpheres) (Math|Transform|MakeTransform _array_element) false)))